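; Base enemy character with sword combat, providing chase, attack, weapon and movement-speed actions.
; Chasing uses AI MoveTo toward the player, attacking on arrival and repeating after a short delay.
; Montage notifies spawn and socket-attach or destroy the sword, while montage endings fire dispatchers for attack, wield and sheathe.
; Functions expose ideal attack and defend ranges, a patrol route, and walk speed selected by movement state.
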(event `self.ReceiveBeginPlay`)

(event `ChasePlayer`
  (`|AIMoveTo` self (0.0 0.0 0.0) (`GameplayStatics.GetPlayerCharacter` 0) 111.0
    (:`OnSuccess`
      (`self.Attack`)
      (`KismetSystemLibrary.Delay` 2.0)
      (`self.ChasePlayer`))))

(event `Attack`
  (`|PlayMontage` (`self.Mesh`) "/Game/Mixamo/RetargettedAnimation/Sword_And_Shield_Slash_Anim_Montage.Sword_And_Shield_Slash_Anim_Montage"
    (:`OnCompleted`
      _)
    (:`OnInterrupted`
      _))
  (`self.OnEndAttack`))

(event `WeildSword`
  (bind _notifyname (`|PlayMontage` (`self.Mesh`) "/Game/Mixamo/RetargettedAnimation/WeildSword_Montage.WeildSword_Montage")
    (:`OnCompleted`
      (`self.OnSuccessWeild`))
    (:`OnNotifyBegin`
      (switch `name` _notifyname
        (:`HoldSword`
          (bind _returnvalue (`|SpawnActorFromClass` "/Game/Weapons/BP_Sword.BP_Sword_C" (`self.GetTransform`) "Undefined" "MultiplyWithRoot" null null))
          (set `self.SwordActor` _returnvalue)
          (`self.K2_AttachToComponent` _returnvalue (`self.Mesh`) "hand_rSocket" "SnapToTarget" "SnapToTarget" "SnapToTarget" true)
          (set `self.IsWeildingSword` true))))))

(event `SheithSword`
  (bind _notifyname (`|PlayMontage` (`self.Mesh`) "/Game/Mixamo/RetargettedAnimation/Sheathing_Sword_Montage.Sheathing_Sword_Montage")
    (:`OnCompleted`
      (`self.OnSheithSword`))
    (:`OnNotifyBegin`
      (switch `name` _notifyname
        (:`DropSword`
          (`self.K2_DestroyActor` (`self.SwordActor`))
          (set `self.IsWeildingSword` false))))))

(fn `GetIdealRange`
  (returns (AttackRadious :type "Float (double-precision)") (DefendRadious :type "Float (double-precision)"))
  (return 150.0 400.0))

(fn `GetPetrolRoute`
  (returns (Route :type "/Game/Blueprint/BP_Patrol Object Reference"))
  (return (`self.PatrolRoute`)))

(fn `SetMovementSpeed`
  (params (Movement :type "/Game/Enums/E_EnemySpeed Enum" :default "NewEnumerator0"))
  (returns (Speed :type "Float (double-precision)"))
  (bind _output_get (set `CharacterMovementComponent.MaxWalkSpeed` (select `/Game/Enums/E_EnemySpeed` Movement :`NewEnumerator1` 150.0 :`NewEnumerator2` 300.0 :`NewEnumerator3` 500.0 :!type "Float (single-precision)") (`self.CharacterMovement`)))
  (return _output_get))

(fn `UserConstructionScript`)